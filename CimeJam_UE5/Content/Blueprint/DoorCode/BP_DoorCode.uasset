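; BP_DoorCode is a door opened through a code prompt.
; Interact creates a WBP_PromptCode widget, passing the code and a reference to the door, and adds it to the viewport.
; OpenDoor plays a timeline that lerps the Cube mesh 300 units down from its current relative location, with no sweep.
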(event Custom|OpenDoor
  (Variables|Default|SetRLoc (Variables|/Script/Engine.SceneComponent|GetRelativeLocation (Variables|Default|GetCube)))
  (bind _alpha (Timeline|Open PlayFromStart)
    (:Update
      (Transformation|SetRelativeLocation (Variables|Default|GetCube) (Math|Vector|Lerp(Vector) (Variables|Default|GetRLoc) (- (Variables|Default|GetRLoc) "0.000000,0.000000,300.000000") _alpha) false false))))

(event EventBeginPlay)

(event Collision|EventActorBeginOverlap
  (params (OtherActor :type Actor%20Object%20Reference)))

(event EventTick
  (params (DeltaSeconds :type Float%20%28single-precision%29)))

(event EventInteract
  (bind _returnvalue (UserInterface|CreateWidget "/Game/Blueprint/UI/WBP_PromptCode.WBP_PromptCode_C" 0 (Variables|Default|GetCode) self))
  (UserInterface|Viewport|AddtoViewport _returnvalue 0))

(fn ConstructionScript)