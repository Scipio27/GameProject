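; BpDoor is a double door that swings open and closed through OpenDoor and CloseDoor events.
; BeginPlay caches the panels' starting rotations and the door location.
; Opening plays a sound and two timelines that rotate StaticMesh and Gauche 90 degrees in opposite yaw directions; closing reverses both.
; Both panels interpolate from the StaticMesh rotation, leaving the stored Gauche rotation and location unused.
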(event Custom|OpenDoor
  (bind _rotd (Variables|Default|GetRotD))
  (bind _rotd_2 (Variables|Default|GetRotD))
  (bind (_roll _pitch _yaw) (Math|Rotator|BreakRotator _rotd))
  (bind (_roll_2 _pitch_2 _yaw_2) (Math|Rotator|BreakRotator _rotd_2))
  ;[0.05127 0.05127 0.05127] NewLockZ
  (Utilities|FlowControl|Sequence
    (:then_0
      (Audio|PlaySoundatLocation "/Game/Son/Door.Door" (Transformation|GetWorldLocation (Variables|Default|GetDefaultSceneRoot)) "0, 0, 0" 1.0 1.0 0.0 0 0 0 0)
      (bind _newtrack_1 (Timeline|Right Play)
        (:Update
          (Transformation|SetRelativeRotation (Variables|Default|GetStaticMesh) (Math|Rotator|Lerp(Rotator) _rotd_2 (Math|Rotator|MakeRotator _roll_2 _pitch_2 (- _yaw_2 -9e+01)) _newtrack_1 true) false false))))
    (:then_1
      (bind _newtrack_1_2 (Timeline|Left Play)
        (:Update
          (Transformation|SetRelativeRotation (Variables|Default|GetGauche) (Math|Rotator|Lerp(Rotator) _rotd (Math|Rotator|MakeRotator _roll _pitch (- _yaw 9e+01)) _newtrack_1_2 true) false false))))))

(event Custom|CloseDoor
  (Utilities|String|Reverse (Variables|Default|GetRight))
  (Utilities|String|Reverse (Variables|Default|GetLeft)))

(event EventBeginPlay
  (Variables|Default|SetLocDoor (Variables|/Script/Engine.SceneComponent|GetRelativeLocation (Variables|Default|GetStaticMesh)))
  (Variables|Default|SetRotG (Variables|/Script/Engine.SceneComponent|GetRelativeRotation (Variables|Default|GetGauche)))
  (Variables|Default|SetRotD (Variables|/Script/Engine.SceneComponent|GetRelativeRotation (Variables|Default|GetStaticMesh))))

(fn ConstructionScript)