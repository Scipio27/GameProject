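; BP_DoorLevier is a double door that swings open once, triggered by levers or a button.
; Verif counts lever calls, calling Invalid on the lever at the first and opening from the second, while Bouton skips the count.
; A DoOnce gates the door sound and two timelines rotating Cube and Gauche 90 degrees in opposite yaw directions.
; Both leaves lerp from Cube's initial rotation; Gauche's saved rotation is unused.
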(event Custom|Verif
  (params (Levier :type BP%20Autre%20Levier%20Object%20Reference))
  (bind _count (Variables|Default|GetCount))
  (bind _rotd (Variables|Default|GetRotD))
  (bind _rotd_2 (Variables|Default|GetRotD))
  (bind (_roll _pitch _yaw) (Math|Rotator|BreakRotator _rotd))
  (bind (_roll_2 _pitch_2 _yaw_2) (Math|Rotator|BreakRotator _rotd_2))
  (Math|Integer|IncrementInt _count
    (:%20%20
      (if (<= _count 1)
        (Default|Invalid Levier)
        (else
          (Utilities|FlowControl|DoOnce false
            (:Completed
              (Utilities|FlowControl|Sequence
                (:then_0
                  (Audio|PlaySoundatLocation "/Game/Son/Door.Door" (Transformation|GetWorldLocation (Variables|Default|GetDefaultSceneRoot)) "0, 0, 0" 1.0 1.0 0.0 0 0 0 0)
                  (bind _alpha (Timeline|Open PlayFromStart)
                    (:Update
                      (Transformation|SetRelativeRotation (Variables|Default|GetCube) (Math|Rotator|Lerp(Rotator) _rotd_2 (Math|Rotator|MakeRotator _roll_2 _pitch_2 (- _yaw_2 -9e+01)) _alpha true) false false))))
                (:then_1
                  (bind _alpha_2 (Timeline|Timeline PlayFromStart)
                    (:Update
                      (Transformation|SetRelativeRotation (Variables|Default|GetGauche) (Math|Rotator|Lerp(Rotator) _rotd (Math|Rotator|MakeRotator _roll _pitch (- _yaw 9e+01)) _alpha_2 true) false false))))))))))))

(event Custom|Bouton
  (bind _rotd (Variables|Default|GetRotD))
  (bind _rotd_2 (Variables|Default|GetRotD))
  (bind (_roll _pitch _yaw) (Math|Rotator|BreakRotator _rotd))
  (bind (_roll_2 _pitch_2 _yaw_2) (Math|Rotator|BreakRotator _rotd_2))
  (Utilities|FlowControl|DoOnce false
    (:Completed
      (Utilities|FlowControl|Sequence
        (:then_0
          (Audio|PlaySoundatLocation "/Game/Son/Door.Door" (Transformation|GetWorldLocation (Variables|Default|GetDefaultSceneRoot)) "0, 0, 0" 1.0 1.0 0.0 0 0 0 0)
          (bind _alpha (Timeline|Open PlayFromStart)
            (:Update
              (Transformation|SetRelativeRotation (Variables|Default|GetCube) (Math|Rotator|Lerp(Rotator) _rotd_2 (Math|Rotator|MakeRotator _roll_2 _pitch_2 (- _yaw_2 -9e+01)) _alpha true) false false))))
        (:then_1
          (bind _alpha_2 (Timeline|Timeline PlayFromStart)
            (:Update
              (Transformation|SetRelativeRotation (Variables|Default|GetGauche) (Math|Rotator|Lerp(Rotator) _rotd (Math|Rotator|MakeRotator _roll _pitch (- _yaw 9e+01)) _alpha_2 true) false false))))))))

(event EventBeginPlay
  (Variables|Default|SetRotD (Variables|/Script/Engine.SceneComponent|GetRelativeRotation (Variables|Default|GetCube)))
  (Variables|Default|SetRotG (Variables|/Script/Engine.SceneComponent|GetRelativeRotation (Variables|Default|GetGauche))))

(event Collision|EventActorBeginOverlap
  (params (OtherActor :type Actor%20Object%20Reference)))

(event EventTick
  (params (DeltaSeconds :type Float%20%28single-precision%29)))

(fn ConstructionScript)