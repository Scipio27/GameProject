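; Pressure plate Blueprint that opens linked doors while the first-person player or a BP_Kadaver stands on it.
; A box overlap raises a counter for each qualifying actor and calls OpenDoor on every entry in DoorRef.
; End overlap lowers the counter and calls CloseDoor on those doors only when it reaches zero or below, so several occupants can share the plate.
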(event OnComponentBeginOverlap(Box)
  (params (OverlappedComponent :type Primitive%20Component%20Object%20Reference) (OtherActor :type Actor%20Object%20Reference) (OtherComp :type Primitive%20Component%20Object%20Reference) (OtherBodyIndex :type Integer) (bFromSweep :type Boolean) (SweepResult :type Hit%20Result%20Structure%20%28by%20ref%29))
  (Utilities|FlowControl|Sequence
    (:then_0
      (Utilities|Casting|CastToBP_FirstPersonCharacter OtherActor))
    (:then_1
      (Utilities|Casting|CastToBP_Kadaver OtherActor)))
  (Math|Integer|IncrementInt (Variables|Default|Getcount)
    (:%20%20
      (for _array_element (Variables|Default|GetDoorRef)
        (Default|OpenDoor _array_element)))))

(event OnComponentEndOverlap(Box)
  (params (OverlappedComponent :type Primitive%20Component%20Object%20Reference) (OtherActor :type Actor%20Object%20Reference) (OtherComp :type Primitive%20Component%20Object%20Reference) (OtherBodyIndex :type Integer))
  (Utilities|FlowControl|Sequence
    (:then_0
      (Utilities|Casting|CastToBP_FirstPersonCharacter OtherActor))
    (:then_1
      (Utilities|Casting|CastToBP_Kadaver OtherActor)))
  (Math|Integer|DecrementInt (Variables|Default|Getcount)
    (:%20%20
      (if (<= (Variables|Default|Getcount) 0)
        (for _array_element (Variables|Default|GetDoorRef)
          (Default|CloseDoor _array_element))))))

(fn ConstructionScript)