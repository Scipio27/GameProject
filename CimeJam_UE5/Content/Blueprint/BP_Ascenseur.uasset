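; BP_Ascenseur is an elevator that, once activated by Interact, raises and lowers its platform in a continuous loop.
; A DoOnce accepts only the first interaction, storing the platform's relative location as the start point.
; The Move timeline lerps the platform to that point plus the Heigh vertical offset.
; On each finish, a FlipFlop alternates reversing and replaying the timeline, with matching up or down sounds.
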(event EventBeginPlay)

(event Collision|EventActorBeginOverlap
  (params (OtherActor :type Actor%20Object%20Reference)))

(event EventTick
  (params (DeltaSeconds :type Float%20%28single-precision%29)))

(event EventInteract
  (bind _move (Variables|Default|GetMove))
  (Utilities|FlowControl|DoOnce false
    (:Completed
      (Variables|Default|SetRLoc (Variables|/Script/Engine.SceneComponent|GetRelativeLocation (Variables|Default|GetPlateforme)))
      (Audio|PlaySoundatLocation "/Game/Son/AscenseurUP.AscenseurUP" (Transformation|GetWorldLocation (Variables|Default|GetPlateforme)) "0, 0, 0" 1.0 1.0 0.0 0 0 0 0)
      (bind _alpha (Timeline|Move PlayFromStart)
        (:Update
          (Transformation|SetRelativeLocation (Variables|Default|GetPlateforme) (Math|Vector|Lerp(Vector) (Variables|Default|GetRLoc) (+ (Variables|Default|GetRLoc) (Math|Vector|MakeVector 0.0 0.0 (Variables|Default|GetHeigh))) _alpha) false false))
        (:Finished
          (Utilities|FlowControl|FlipFlop
            (:A
              (Components|Timeline|ReversefromEnd _move)
              (Audio|PlaySoundatLocation "/Game/Son/AscenseurDown.AscenseurDown" (Transformation|GetWorldLocation (Variables|Default|GetPlateforme)) "0, 0, 0" 1.0 1.0 0.0 0 0 0 0))
            (:B
              (Components|Timeline|PlayfromStart _move)
              (Audio|PlaySoundatLocation "/Game/Son/AscenseurUP.AscenseurUP" (Transformation|GetWorldLocation (Variables|Default|GetPlateforme)) "0, 0, 0" 1.0 1.0 0.0 0 0 0 0))))))))

(fn ConstructionScript)