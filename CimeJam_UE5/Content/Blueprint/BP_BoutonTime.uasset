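; Timed puzzle button that succeeds only when pressed while its digit appears in the player's battery percentage or timer seconds, as set by the Battery flag.
; Interact plays a sound and the Press timeline, with a FlipFlop reversing it before VerifDigit compares Value to the readout's first two characters.
; A match turns the cube valid, notifies the door and stays locked; a miss turns it invalid, subtracts timer seconds and re-arms.
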(event EventBeginPlay
  (bind _asbp_first_person_character (Utilities|Casting|CastToBP_FirstPersonCharacter (Game|GetPlayerCharacter 0)))
  (Variables|Default|SetPlayerRef _asbp_first_person_character)
  (Variables|Default|SetLocRef (Transformation|GetActorLocation)))

(event Collision|EventActorBeginOverlap
  (params (OtherActor :type Actor%20Object%20Reference)))

(event EventTick
  (params (DeltaSeconds :type Float%20%28single-precision%29)))

(event EventInteract
  (bind _locref (Variables|Default|GetLocRef))
  (bind _playerref (Variables|Default|GetPlayerRef))
  (bind _chronoref (Variables|/Game/FirstPerson/Blueprints/BP_FirstPersonCharacter.BP_FirstPersonCharacter_C|GetChronoRef _playerref))
  (if (Variables|Default|GetCanActivate)
    (Variables|Default|SetCanActivate false)
    (Audio|PlaySoundatLocation "/Game/Son/Switch.Switch" (Transformation|GetActorLocation) "0, 0, 0" 1.0 1.0 0.0 0 0 0 0)
    (bind _alpha (Timeline|Press PlayFromStart)
      (:Update
        (Transformation|SetActorLocation (Math|Vector|Lerp(Vector) _locref (- _locref "5.000000,0.000000,0.000000") _alpha) false false))
      (:Finished
        (Utilities|FlowControl|FlipFlop
          (:A
            (Components|Timeline|ReversefromEnd (Variables|Default|GetPress)))
          (:B
            (if (CallFunction|VerifDigit)
              (Rendering|Material|SetMaterial (Variables|Default|GetCube) 0 "/Game/Blueprint/Material/M_Valide.M_Valide")
              (Default|Bouton (Variables|Default|GetDoorRef))
              (else
                (Variables|/Game/Blueprint/UI/WBP_Chrono.WBP_Chrono_C|SetSeconds _chronoref (- (Variables|/Game/Blueprint/UI/WBP_Chrono.WBP_Chrono_C|GetSeconds _chronoref) 5))
                (Rendering|Material|SetMaterial (Variables|Default|GetCube) 0 "/Game/Blueprint/Material/M_Invalide.M_Invalide")
                (Variables|Default|SetCanActivate true)))))))))

(fn ConstructionScript)

(fn VerifDigit
  (bind _value (Variables|Default|GetValue))
  (bind _value_2 (Variables|Default|GetValue))
  (if (Variables|Default|GetBattery)
    (return (or (== (Utilities|Array|Get(acopy) (Utilities|String|GetCharacterArrayfromString (Utilities|String|ToString(Integer) (Variables|/Game/Blueprint/UI/WBP_Batterie.WBP_Batterie_C|GetNumPercent (Variables|/Game/FirstPerson/Blueprints/BP_FirstPersonCharacter.BP_FirstPersonCharacter_C|GetBatterieRef (Variables|Default|GetPlayerRef)))))) _value_2) (== _value_2 (Utilities|Array|Get(acopy) (Utilities|String|GetCharacterArrayfromString (Utilities|String|ToString(Integer) (Variables|/Game/Blueprint/UI/WBP_Batterie.WBP_Batterie_C|GetNumPercent (Variables|/Game/FirstPerson/Blueprints/BP_FirstPersonCharacter.BP_FirstPersonCharacter_C|GetBatterieRef (Variables|Default|GetPlayerRef))))) 1))))
    (else
      (return (or (== (Utilities|Array|Get(acopy) (Utilities|String|GetCharacterArrayfromString (Utilities|String|ToString(Integer) (Variables|/Game/Blueprint/UI/WBP_Chrono.WBP_Chrono_C|GetSeconds (Variables|/Game/FirstPerson/Blueprints/BP_FirstPersonCharacter.BP_FirstPersonCharacter_C|GetChronoRef (Variables|Default|GetPlayerRef)))))) _value) (== _value (Utilities|Array|Get(acopy) (Utilities|String|GetCharacterArrayfromString (Utilities|String|ToString(Integer) (Variables|/Game/Blueprint/UI/WBP_Chrono.WBP_Chrono_C|GetSeconds (Variables|/Game/FirstPerson/Blueprints/BP_FirstPersonCharacter.BP_FirstPersonCharacter_C|GetChronoRef (Variables|Default|GetPlayerRef))))) 1)))))))