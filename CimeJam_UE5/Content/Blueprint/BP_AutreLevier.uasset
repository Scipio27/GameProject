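; Interactable lever that tilts once with a sound, then notifies its linked door.
; Interact uses a DoOnce and a timeline to rotate the cube 60 degrees in pitch.
; When the timeline finishes, a FlipFlop calls the door's Verif for trap levers (Piege) or Bouton otherwise, skipping the next finish.
; The Invalid event reverses the tilt and subtracts 10 from the player's chrono seconds.
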(event Custom|Invalid
  (bind _playerref (Variables|Default|GetPlayerRef))
  (bind _chronoref (Variables|/Game/FirstPerson/Blueprints/BP_FirstPersonCharacter.BP_FirstPersonCharacter_C|GetChronoRef _playerref))
  (Components|Timeline|ReversefromEnd (Variables|Default|GetMove))
  (Variables|/Game/Blueprint/UI/WBP_Chrono.WBP_Chrono_C|SetSeconds _chronoref (- (Variables|/Game/Blueprint/UI/WBP_Chrono.WBP_Chrono_C|GetSeconds _chronoref) 10)))

(event EventBeginPlay
  (bind _asbp_first_person_character (Utilities|Casting|CastToBP_FirstPersonCharacter (Game|GetPlayerCharacter 0)))
  (Variables|Default|SetPlayerRef _asbp_first_person_character))

(event Collision|EventActorBeginOverlap
  (params (OtherActor :type Actor%20Object%20Reference)))

(event EventTick
  (params (DeltaSeconds :type Float%20%28single-precision%29)))

(event EventInteract
  (bind _doorref (Variables|Default|GetDoorRef))
  (Utilities|FlowControl|DoOnce false
    (:Completed
      (Variables|Default|SetRotRef (Transformation|GetWorldRotation (Variables|Default|GetCube)))
      (Audio|PlaySoundatLocation "/Game/Son/Lever.Lever" (Transformation|GetWorldLocation (Variables|Default|GetStaticMesh)) "0, 0, 0" 1.0 1.0 0.0 0 0 0 0)
      (bind _alpha (Timeline|Move PlayFromStart)
        (:Update
          (Transformation|SetWorldRotation (Variables|Default|GetCube) (Math|Rotator|Lerp(Rotator) (Variables|Default|GetRotRef) (Math|Rotator|MakeRotator (.Roll (Math|Rotator|BreakRotator (Variables|Default|GetRotRef))) (+ (.Pitch (Math|Rotator|BreakRotator (Variables|Default|GetRotRef))) -6e+01) (.Yaw (Math|Rotator|BreakRotator (Variables|Default|GetRotRef)))) _alpha true) false false))
        (:Finished
          (Utilities|FlowControl|FlipFlop
            (:A
              (if (Variables|Default|GetPiege)
                (Default|Verif _doorref self)
                (else
                  (Default|Bouton _doorref))))))))))

(fn ConstructionScript)