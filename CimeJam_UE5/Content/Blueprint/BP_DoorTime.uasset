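; BP_DoorTime is a double door whose two leaves, Cube and StaticMesh, swing 90 degrees in opposite yaw directions.
; BeginPlay caches each leaf's starting relative rotation.
; OpenCloseDoor plays a door sound and starts two timelines that lerp the leaves open from those rotations.
; The separate Reverse event runs both timelines back from the end to close them, without triggering the sound.
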(event Custom|OpenCloseDoor
  (bind _rotg (Variables|Default|GetRotG))
  (bind _rotd (Variables|Default|GetRotD))
  (bind (_roll _pitch _yaw) (Math|Rotator|BreakRotator _rotg))
  (bind (_roll_2 _pitch_2 _yaw_2) (Math|Rotator|BreakRotator _rotd))
  (Utilities|FlowControl|Sequence
    (:then_0
      (Audio|PlaySoundatLocation "/Game/Son/Door.Door" (Transformation|GetWorldLocation (Variables|Default|GetDefaultSceneRoot)) "0, 0, 0" 1.0 1.0 0.0 0 0 0 0)
      (bind _alpha (Timeline|Move PlayFromStart)
        (:Update
          (Transformation|SetRelativeRotation (Variables|Default|GetCube) (Math|Rotator|Lerp(Rotator) _rotg (Math|Rotator|MakeRotator _roll _pitch (- _yaw -9e+01)) _alpha true) false false))))
    (:then_1
      (bind _alpha_2 (Timeline|Timeline PlayFromStart)
        (:Update
          (Transformation|SetRelativeRotation (Variables|Default|GetStaticMesh) (Math|Rotator|Lerp(Rotator) _rotd (Math|Rotator|MakeRotator _roll_2 _pitch_2 (- _yaw_2 9e+01)) _alpha_2 true) false false))))))

(event Custom|Reverse
  (bind _rotg (Variables|Default|GetRotG))
  (bind _rotd (Variables|Default|GetRotD))
  (bind (_roll _pitch _yaw) (Math|Rotator|BreakRotator _rotg))
  (bind (_roll_2 _pitch_2 _yaw_2) (Math|Rotator|BreakRotator _rotd))
  (Utilities|FlowControl|Sequence
    (:then_0
      (bind _alpha (Timeline|Move ReverseFromEnd)
        (:Update
          (Transformation|SetRelativeRotation (Variables|Default|GetCube) (Math|Rotator|Lerp(Rotator) _rotg (Math|Rotator|MakeRotator _roll _pitch (- _yaw -9e+01)) _alpha true) false false))))
    (:then_1
      (bind _alpha_2 (Timeline|Timeline ReverseFromEnd)
        (:Update
          (Transformation|SetRelativeRotation (Variables|Default|GetStaticMesh) (Math|Rotator|Lerp(Rotator) _rotd (Math|Rotator|MakeRotator _roll_2 _pitch_2 (- _yaw_2 9e+01)) _alpha_2 true) false false))))))

(event EventBeginPlay
  (Variables|Default|SetRotG (Variables|/Script/Engine.SceneComponent|GetRelativeRotation (Variables|Default|GetCube)))
  (Variables|Default|SetRotD (Variables|/Script/Engine.SceneComponent|GetRelativeRotation (Variables|Default|GetStaticMesh))))

(event Collision|EventActorBeginOverlap
  (params (OtherActor :type Actor%20Object%20Reference)))

(event EventTick
  (params (DeltaSeconds :type Float%20%28single-precision%29)))

(fn ConstructionScript)