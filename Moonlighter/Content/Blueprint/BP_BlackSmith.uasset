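; BP_BlackSmith is a blacksmith actor that acts as a crafting zone for the first-person player character.
; On begin overlap it sets the character's Craft flag and calls Toggle on the CraftMenu held by BP_PlayerController.
; On end overlap it only clears the Craft flag, leaving the menu untouched.
; A disconnected branch that would create and display WBP_BlackSmith never runs.
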(event EventBeginPlay)

(event Collision|EventActorBeginOverlap
  (params (OtherActor :type Actor%20Object%20Reference))
  (bind _asfirst_person_character (Utilities|Casting|CastToFirstPersonCharacter OtherActor))
  (Variables|/Game/FirstPersonBP/Blueprints/FirstPersonCharacter.FirstPersonCharacter_C|Setcraft _asfirst_person_character true)
  (bind _asbp_player_controller (Utilities|Casting|CastToBP_PlayerController (Game|GetPlayerController 0)))
  (Default|Toggle (Variables|/Game/Blueprint/BP_PlayerController.BP_PlayerController_C|GetCraftMenu _asbp_player_controller)))

(event Collision|EventActorEndOverlap
  (params (OtherActor :type Actor%20Object%20Reference))
  (bind _asfirst_person_character (Utilities|Casting|CastToFirstPersonCharacter OtherActor))
  (Variables|/Game/FirstPersonBP/Blueprints/FirstPersonCharacter.FirstPersonCharacter_C|Setcraft _asfirst_person_character false))

(fn ConstructionScript)