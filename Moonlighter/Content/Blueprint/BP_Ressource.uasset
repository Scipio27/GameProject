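; BP_Ressource is a resource pickup actor that goes into the player's inventory when interacted with.
; Interact adds one item of the actor's own class to the player's BPInventoryComponent, refreshes the craft menu inventory through BP_PlayerController (player 0), then destroys the actor.
; A hit on the Mesh component turns off physics simulation on the Sphere component.
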(event OnComponentHit(Mesh)
  (params (HitComponent :type Primitive%20Component%20Object%20Reference) (OtherActor :type Actor%20Object%20Reference) (OtherComp :type Primitive%20Component%20Object%20Reference) (NormalImpulse :type Vector :default "0, 0, 0") (Hit :type Hit%20Result%20Structure%20%28by%20ref%29))
  (Physics|SetSimulatePhysics (Variables|Default|GetSphere) false))

(event EventBeginPlay)

(event Collision|EventActorBeginOverlap
  (params (OtherActor :type Actor%20Object%20Reference)))

(event EventTick
  (params (DeltaSeconds :type Float%20%28single-precision%29)))

(event EventInteract
  (params (Player :type First%20Person%20Character%20Object%20Reference))
  (Default|AddtoInventory (Variables|/Game/FirstPersonBP/Blueprints/FirstPersonCharacter.FirstPersonCharacter_C|GetBP_InventoryComponent Player) (Utilities|GetClass self) 1)
  (bind _asbp_player_controller (Utilities|Casting|CastToBP_PlayerController (Game|GetPlayerController 0)))
  (Default|RefreshInventory (Variables|/Game/Blueprint/WBP_CraftMenu.WBP_CraftMenu_C|GetWBP_Craft (Variables|/Game/Blueprint/BP_PlayerController.BP_PlayerController_C|GetCraftMenu _asbp_player_controller)))
  (Actor|DestroyActor))

(fn ConstructionScript)