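; Inventory component that tracks item quantities in a map, with functions to add, query and remove items.
; AddToInventory sums onto the stored count, clamped to a fixed stack range, and always returns false.
; QueryInventory reports the held count and whether it covers a requested quantity.
; RemoveInventory uses that query before subtracting, leaving emptied items in the map at zero.
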(event EventBeginPlay)

(event EventTick
  (params (DeltaSeconds :type Float%20%28single-precision%29)))

(fn AddtoInventory
  (params (Item%20to%20add :type BP%20Ressource%20Class%20Reference) (Quantity :type Integer))
  (Utilities|Map|Add (Variables|Default|GetInventory) Item%20to%20add (Math|Integer|Clamp(Integer) (+ Quantity (.Value (Utilities|Map|Find (Variables|Default|GetInventory) Item%20to%20add))) 0 99))
  (return false))

(fn QueryInventory
  (params (Item :type BP%20Ressource%20Class%20Reference) (Quantity :type Integer))
  (bind _inventory (Variables|Default|GetInventory))
  (bind (_value _returnvalue) (Utilities|Map|Find _inventory Item))
  (if (and (<= Quantity _value) _returnvalue)
    (return _value true)
    (else
      (return _value false))))

(fn RemoveInventory
  (params (Item%20to%20remove :type BP%20Ressource%20Class%20Reference) (Quantity :type Integer))
  (bind (_outputquantity _success) (CallFunction|QueryInventory Item%20to%20remove Quantity))
  (if _success
    (Utilities|Map|Add (Variables|Default|GetInventory) Item%20to%20remove (- _outputquantity Quantity))
    (return true)
    (else
      (return false))))