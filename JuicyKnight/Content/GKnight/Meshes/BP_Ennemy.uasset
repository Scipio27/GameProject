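; BP_Ennemy is an enemy character that carries a world-space widget and can die into a physics ragdoll.
; Each tick it rotates the widget, while valid, to face the first-person player's camera as a billboard.
; The Death function turns on mesh physics, disables movement, then destroys the widget and, only if that widget was valid, the capsule component.
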(event EventBeginPlay)

(event Collision|EventActorBeginOverlap
  (params (OtherActor :type Actor%20Object%20Reference)))

(event EventTick
  (params (DeltaSeconds :type Float%20%28single-precision%29))
  (bind _widget (Variables|Default|GetWidget))
  (bind _asfirst_person_character (Utilities|Casting|CastToFirstPersonCharacter (Game|GetPlayerCharacter 0)))
  (Utilities|IsValid _widget
    (:Is%20Valid
      (Transformation|SetWorldRotation (Variables|Default|GetWidget) (Math|Rotator|FindLookatRotation (Transformation|GetWorldLocation _widget) (Transformation|GetWorldLocation (Variables|/Game/FPSwordAndShield/Blueprints/FirstPersonCharacter.FirstPersonCharacter_C|GetFirstPersonCamera _asfirst_person_character))) false false))))

(fn ConstructionScript)

(fn Death
  (bind _widget (Variables|Default|GetWidget))
  (bind _capsulecomponent (Variables|Collision|GetCapsuleComponent))
  (Physics|SetSimulatePhysics (Variables|Character|GetMesh) true)
  (Pawn|Components|CharacterMovement|DisableMovement (Variables|Character|GetCharacterMovement))
  (Utilities|IsValid _widget
    (:Is%20Valid
      (Components|DestroyComponent _widget)
      (Utilities|IsValid _capsulecomponent
        (:Is%20Valid
          (Components|DestroyComponent _capsulecomponent))))))