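; AI controller for an enemy that runs the BT_Ennemy behavior tree on begin play and tracks the player through AI perception.
; When a FirstPersonCharacter is sensed, it is written to the TargetRef blackboard key and any pending clear timer is cancelled.
; When sensing is lost, a three-second timer starts and then clears TargetRef, giving a short memory of the target.
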(event OnTargetPerceptionUpdated(AIPerception)
  (params (Actor :type Actor%20Object%20Reference) (Stimulus :type AI%20Stimulus%20Structure))
  (bind _asfirst_person_character (Utilities|Casting|CastToFirstPersonCharacter Actor))
  (if (.bsuccessfullysensed Stimulus)
    (AI|Components|Blackboard|SetValueasObject (Variables|Default|GetBlackboard) (Utilities|String|StringToName "TargetRef") _asfirst_person_character)
    (if (Utilities|Time|IsValidTimerHandle (Variables|Default|GettimerHandleClear))
      (Utilities|Time|ClearandInvalidateTimerbyHandle (Variables|Default|GettimerHandleClear)))
    (else
      (bind _returnvalue (Utilities|Time|SetTimerbyEvent (delegate Custom|Clear) 3.0))
      (Variables|Default|SettimerHandleClear _returnvalue))))

(event Custom|Clear
  (AI|Components|Blackboard|ClearValue (Variables|Default|GetBlackboard) (Utilities|String|StringToName "TargetRef")))

(event EventBeginPlay
  (AI|RunBehaviorTree "/Game/GKnight/Meshes/BT_Ennemy.BT_Ennemy"))

(event EventTick
  (params (DeltaSeconds :type Float%20%28single-precision%29)))

(fn ConstructionScript)