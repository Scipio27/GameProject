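; BP_Cell_Door is an interactable dungeon cell door that opens and closes only when KeyUsable is set and the instigator has the key.
; A successful interaction removes the on-screen key widget and uses a FlipFlop to play or reverse the Open timeline, which yaws the door mesh up to 110 degrees.
; While KeyUsable is set, entering the trigger box shows a door widget, removed on exit, and interacting keyless shows a key-door widget.
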(event OnComponentBeginOverlap(Box)
  (params (OverlappedComponent :type Primitive%20Component%20Object%20Reference) (OtherActor :type Actor%20Object%20Reference) (OtherComp :type Primitive%20Component%20Object%20Reference) (OtherBodyIndex :type Integer) (bFromSweep :type Boolean) (SweepResult :type Hit%20Result%20Structure%20%28by%20ref%29))
  (if (Variables|Default|GetKeyUsable)
    (Utilities|Casting|CastToFirstPersonCharacter OtherActor)
    (bind _returnvalue (UserInterface|CreateWidget "/Game/FPSwordAndShield/Blueprints/WBP_Door.WBP_Door_C" (Game|GetPlayerController 0)))
    (UserInterface|Viewport|AddtoViewport _returnvalue 0)))

(event OnComponentEndOverlap(Box)
  (params (OverlappedComponent :type Primitive%20Component%20Object%20Reference) (OtherActor :type Actor%20Object%20Reference) (OtherComp :type Primitive%20Component%20Object%20Reference) (OtherBodyIndex :type Integer))
  (Utilities|IsValid (stale OnComponentBeginOverlap(Box) _returnvalue)
    (:Is%20Valid
      (Widget|RemovefromParent (stale OnComponentBeginOverlap(Box) _returnvalue)))))

(event Collision|EventActorBeginOverlap
  (params (OtherActor :type Actor%20Object%20Reference)))

(event EventTick
  (params (DeltaSeconds :type Float%20%28single-precision%29)))

(event EventInteraction
  (params (Instigator :type First%20Person%20Character%20Object%20Reference))
  (if (and (Variables|/Game/FPSwordAndShield/Blueprints/FirstPersonCharacter.FirstPersonCharacter_C|GethaveKey Instigator) (Variables|Default|GetKeyUsable))
    (Variables|Default|Setuse true)
    ;[1 1 1] ça marche
    (bind _foundwidgets (Widget|GetAllWidgetsOfClass "/Game/FPSwordAndShield/Blueprints/WBP_Key.WBP_Key_C" true))
    (Widget|RemovefromParent (Utilities|Array|Get(acopy) _foundwidgets))
    (Utilities|FlowControl|FlipFlop
      (:A
        (bind _ouverture (Timeline|Open Play)
          (:Update
            (Transformation|SetRelativeRotation (Variables|Default|GetSM_Cell_Door) (Math|Rotator|MakeRotator 0.0 0.0 (* _ouverture 1.1e+02)) false false))))
      (:B
        (Timeline|Open Reverse)))
    (elif (Variables|Default|GetKeyUsable)
      (bind _returnvalue (UserInterface|CreateWidget "/Game/FPSwordAndShield/Blueprints/WBP_KeyDoor.WBP_KeyDoor_C" (Game|GetPlayerController 0)))
      (UserInterface|Viewport|AddtoViewport _returnvalue 0))))

(fn ConstructionScript)