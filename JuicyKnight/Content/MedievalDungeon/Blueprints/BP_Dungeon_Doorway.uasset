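; BP_Dungeon_Doorway is a double dungeon door that stays shut until the enemy's health is depleted.
; BeginPlay caches a single BP_Ennemy actor, whose health gates the Interaction event.
; Interaction uses a FlipFlop to play or reverse the Open timeline, yawing both leaves in opposite directions by Angle.
; A box trigger shows the WBP_Door widget while the FirstPersonCharacter overlaps it.
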(event OnComponentBeginOverlap(Box)
  (params (OverlappedComponent :type Primitive%20Component%20Object%20Reference) (OtherActor :type Actor%20Object%20Reference) (OtherComp :type Primitive%20Component%20Object%20Reference) (OtherBodyIndex :type Integer) (bFromSweep :type Boolean) (SweepResult :type Hit%20Result%20Structure%20%28by%20ref%29))
  (Utilities|Casting|CastToFirstPersonCharacter OtherActor)
  (bind _returnvalue (UserInterface|CreateWidget "/Game/FPSwordAndShield/Blueprints/WBP_Door.WBP_Door_C" (Game|GetPlayerController 0)))
  (UserInterface|Viewport|AddtoViewport _returnvalue 0))

(event OnComponentEndOverlap(Box)
  (params (OverlappedComponent :type Primitive%20Component%20Object%20Reference) (OtherActor :type Actor%20Object%20Reference) (OtherComp :type Primitive%20Component%20Object%20Reference) (OtherBodyIndex :type Integer))
  (Utilities|Casting|CastToFirstPersonCharacter OtherActor)
  (Widget|RemovefromParent (stale OnComponentBeginOverlap(Box) _returnvalue)))

(event EventBeginPlay
  (bind _returnvalue (Actor|GetActorOfClass "/Game/GKnight/Meshes/BP_Ennemy.BP_Ennemy_C"))
  (Variables|Default|Setenemy _returnvalue))

(event Collision|EventActorBeginOverlap
  (params (OtherActor :type Actor%20Object%20Reference)))

(event EventTick
  (params (DeltaSeconds :type Float%20%28single-precision%29)))

(event EventInteraction
  (params (Instigator :type First%20Person%20Character%20Object%20Reference))
  (if (<= (Variables|/Game/GKnight/Meshes/BP_Ennemy.BP_Ennemy_C|Gethealth (Variables|Default|Getenemy)) 0.0)
    (Utilities|FlowControl|FlipFlop
      (:A
        (bind _rotationvalue (Timeline|Open Play)
          (:Update
            (Transformation|SetRelativeRotation (Variables|Default|GetSM_DoorWay_Large_Door_Left) (Math|Rotator|MakeRotator 0.0 0.0 (* _rotationvalue (Variables|Default|Getangle))) false false)
            (Transformation|SetRelativeRotation (Variables|Default|GetSM_DoorWay_Large_Door_Right) (Math|Rotator|MakeRotator 0.0 0.0 (- 0.0 (* _rotationvalue (Variables|Default|Getangle)))) false false))))
      (:B
        (Timeline|Open Reverse)))))

(fn ConstructionScript)