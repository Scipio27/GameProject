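; Anim notify state for the player's sword attack that detects hits and damages BP_Ennemy during the animation window.
; Each tick box-traces at SwordSocket and spawns a Niagara effect looked up by physical material name, at the actor's location for "Enemy" surfaces.
; The FirstPersonCharacter's Hit flag limits damage to one hit, with no reset here.
; Damage is skipped while Blocking, and zero health triggers Death.
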(fn ReceivedNotifyTick
  (params (MeshComp :type Skeletal%20Mesh%20Component%20Object%20Reference) (Animation :type Anim%20Sequence%20Base%20Object%20Reference) (FrameDeltaTime :type Float%20%28single-precision%29))
  (bind _returnvalue (Transformation|GetSocketLocation MeshComp "SwordSocket"))
  (bind (_outhit _returnvalue_2) (Collision|BoxTraceByChannel MeshComp _returnvalue _returnvalue "10.000000,10.000000,85.000000" (Transformation|GetSocketRotation MeshComp "SwordSocket") "TraceTypeQuery1" false 0 "None"))
  (if _returnvalue_2
    (Niagara|SpawnSystematLocation MeshComp (.Value (Utilities|Map|Find (Variables|Default|GetNiagara) (Utilities|GetDisplayName (.PhysMat (Collision|BreakHitResult _outhit))))) (select (== (Utilities|GetDisplayName (.PhysMat (Collision|BreakHitResult _outhit))) "Enemy") (Transformation|GetActorLocation (.HitActor (Collision|BreakHitResult _outhit))) (Transformation|GetSocketLocation MeshComp "SwordSocket")) (Transformation|GetSocketRotation MeshComp "SwordSocket"))
    (bind _asbp_ennemy (Utilities|Casting|CastToBP_Ennemy (.HitActor (Collision|BreakHitResult _outhit))))
    (bind _returnvalue_3 (Actor|GetActorOfClass MeshComp "/Game/FPSwordAndShield/Blueprints/FirstPersonCharacter.FirstPersonCharacter_C"))
    (if (not (Variables|/Game/FPSwordAndShield/Blueprints/FirstPersonCharacter.FirstPersonCharacter_C|Gethit _returnvalue_3))
      (Variables|/Game/FPSwordAndShield/Blueprints/FirstPersonCharacter.FirstPersonCharacter_C|Sethit _returnvalue_3 true)
      (if (Variables|/Game/FPSwordAndShield/Blueprints/FirstPersonCharacter.FirstPersonCharacter_C|GetBlocking _returnvalue_3)
        _
        (else
          (Variables|/Game/GKnight/Meshes/BP_Ennemy.BP_Ennemy_C|Sethealth _asbp_ennemy (- (Variables|/Game/GKnight/Meshes/BP_Ennemy.BP_Ennemy_C|Gethealth _asbp_ennemy) 25.0))))
      (if (<= (Variables|/Game/GKnight/Meshes/BP_Ennemy.BP_Ennemy_C|Gethealth _asbp_ennemy) 0.0)
        (Default|Death _asbp_ennemy))
      (return false))))

(fn ReceivedNotifyBegin
  (params (MeshComp :type Skeletal%20Mesh%20Component%20Object%20Reference) (Animation :type Anim%20Sequence%20Base%20Object%20Reference) (TotalDuration :type Float%20%28single-precision%29))
  (return false))