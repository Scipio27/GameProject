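; BP_State_HitEnemy is an anim notify state that lets enemy attacks damage the first-person player.
; Each tick box-traces at the mesh's hand_r socket on the Visibility channel, with debug drawing.
; A player hit loses Health, less when Blocking, and at zero teleports to Spawn with Health restored.
; A Hit flag prevents repeat damage, set on the BP_Ennemy found by GetActorOfClass rather than the mesh owner.
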(fn ReceivedNotifyTick
  (params (MeshComp :type Skeletal%20Mesh%20Component%20Object%20Reference) (Animation :type Anim%20Sequence%20Base%20Object%20Reference) (FrameDeltaTime :type Float%20%28single-precision%29) (EventReference :type Anim%20Notify%20Event%20Reference%20Structure%20%28by%20ref%29))
  (bind _returnvalue (Transformation|GetSocketLocation MeshComp "hand_r"))
  (bind (_outhit _returnvalue_2) (Collision|BoxTraceByChannel MeshComp _returnvalue _returnvalue "10.000000,10.000000,85.000000" (Transformation|GetSocketRotation MeshComp "hand_r") "TraceTypeQuery1" false 0 "ForDuration"))
  (if _returnvalue_2
    (bind _asfirst_person_character (Utilities|Casting|CastToFirstPersonCharacter (.HitActor (Collision|BreakHitResult _outhit))))
    (bind _returnvalue_3 (Actor|GetActorOfClass MeshComp "/Game/GKnight/Meshes/BP_Ennemy.BP_Ennemy_C"))
    (if (not (Variables|/Game/GKnight/Meshes/BP_Ennemy.BP_Ennemy_C|Gethit _returnvalue_3))
      (Variables|/Game/GKnight/Meshes/BP_Ennemy.BP_Ennemy_C|Sethit _returnvalue_3 true)
      (if (Variables|/Game/FPSwordAndShield/Blueprints/FirstPersonCharacter.FirstPersonCharacter_C|GetBlocking _asfirst_person_character)
        (Variables|/Game/FPSwordAndShield/Blueprints/FirstPersonCharacter.FirstPersonCharacter_C|Sethealth _asfirst_person_character (- (Variables|/Game/FPSwordAndShield/Blueprints/FirstPersonCharacter.FirstPersonCharacter_C|Gethealth _asfirst_person_character) 1e+01))
        (else
          (Variables|/Game/FPSwordAndShield/Blueprints/FirstPersonCharacter.FirstPersonCharacter_C|Sethealth _asfirst_person_character (- (Variables|/Game/FPSwordAndShield/Blueprints/FirstPersonCharacter.FirstPersonCharacter_C|Gethealth _asfirst_person_character) 5e+01))))
      (if (<= (Variables|/Game/FPSwordAndShield/Blueprints/FirstPersonCharacter.FirstPersonCharacter_C|Gethealth _asfirst_person_character) 0.0)
        (Transformation|SetActorLocation _asfirst_person_character (Variables|/Game/FPSwordAndShield/Blueprints/FirstPersonCharacter.FirstPersonCharacter_C|Getspawn _asfirst_person_character) false true)
        (Variables|/Game/FPSwordAndShield/Blueprints/FirstPersonCharacter.FirstPersonCharacter_C|Sethealth _asfirst_person_character 1e+02))
      (return false))))